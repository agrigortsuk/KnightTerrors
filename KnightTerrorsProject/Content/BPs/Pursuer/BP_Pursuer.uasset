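; BP_Pursuer is an enemy character that patrols randomly, chases the player on sight and damages them on contact.
; A self-restarting AIMoveTo loop roams to nearby navigable points, switching to a faster chase of player 0 while IsSensing is set.
; PawnSensing sets that flag, and a retriggerable delay clears it shortly after BP_Person sightings stop.
; DamageCollisionBox overlaps apply DirectDamage to BP_Person, gated by a short cooldown.
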(event OnSeePawn(PawnSensing)
  (params (Pawn :type Pawn%20Object%20Reference))
  ;[1 1 1] Detecting Player
  (Variables|Default|SetIsSensing true)
  (Utilities|Casting|CastToBP_Person Pawn)
  (CallFunction|ChasePlayer)
  (Utilities|FlowControl|RetriggerableDelay 0.2)
  (Variables|Default|SetIsSensing false))

(event OnComponentBeginOverlap(DamageCollisionBox)
  (params (OverlappedComponent :type Primitive%20Component%20Object%20Reference) (OtherActor :type Actor%20Object%20Reference) (OtherComp :type Primitive%20Component%20Object%20Reference) (OtherBodyIndex :type Integer) (bFromSweep :type Boolean) (SweepResult :type Hit%20Result%20Structure%20%28by%20ref%29))
  ;[1 1 1] Attacking Player on Overlap
  (if (not (Variables|Default|GetIsAttacking))
    (bind _asbp_person (Utilities|Casting|CastToBP_Person OtherActor))
    (Variables|Default|SetIsAttacking true)
    (Game|Damage|ApplyDamage _asbp_person (Variables|Default|GetDirectDamage) 0 0)
    (Utilities|FlowControl|Delay 0.3)
    (Variables|Default|SetIsAttacking false)))

(event Custom|MoveToRandomLocation
  ;[1 1 1] Random Patrol Path
  (if (Variables|Default|GetIsSensing)
    (CallFunction|ChasePlayer)
    (else
      (Variables|/Script/Engine.CharacterMovementComponent|SetMaxWalkSpeed (Variables|Character|GetCharacterMovement self) 4e+02)
      (bind _randomlocation (Class|NavigationSystemV1|GetRandomLocationinNavigableRadius (Transformation|GetActorLocation) 1.5e+03 0 0))
      (AI|AIMoveTo self _randomlocation 0 5.0 false
        (:OnSuccess
          _)
        (:OnFail
          _))
      (Utilities|FlowControl|Delay 0.2)
      (CallFunction|MovetoRandomLocation))))

(event Custom|ChasePlayer
  ;[1 1 1] Chasing Player
  (if (Variables|Default|GetIsSensing)
    (Variables|/Script/Engine.CharacterMovementComponent|SetMaxWalkSpeed (Variables|Character|GetCharacterMovement self) 5e+02)
    (AI|AIMoveTo self "0, 0, 0" (Game|GetPlayerCharacter 0) 5.0 false
      (:OnSuccess
        _)
      (:OnFail
        _))
    (CallFunction|MovetoRandomLocation)))

(event EventBeginPlay
  ;[1 1 1] init
  (CallFunction|MovetoRandomLocation))

(fn ConstructionScript)