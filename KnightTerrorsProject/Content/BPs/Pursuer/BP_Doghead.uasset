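; BP_Doghead is a pursuer enemy that damages the player and imprisons them in a cell on contact.
; Overlapping its DamageCollisionBox with a BP_Person applies DirectDamage and randomly teleports the player pawn to one of two hardcoded locations, guarded by a briefly held IsAttacking flag.
; Tick only casts the player pawn.
; Trail-point following via AIMoveTo and a jumpscare camera-and-animation sequence are present but disconnected.
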(event OnComponentBeginOverlap(DamageCollisionBox)
  (params (OverlappedComponent :type Primitive%20Component%20Object%20Reference) (OtherActor :type Actor%20Object%20Reference) (OtherComp :type Primitive%20Component%20Object%20Reference) (OtherBodyIndex :type Integer) (bFromSweep :type Boolean) (SweepResult :type Hit%20Result%20Structure%20%28by%20ref%29))
  (bind _returnvalue (Game|Player|GetPlayerPawn 0))
  ;[1 1 1] Damage and imprison player in cell
  (if (not (Variables|Default|GetIsAttacking))
    (bind _asbp_person (Utilities|Casting|CastToBP_Person OtherActor))
    (Variables|Default|SetIsAttacking true)
    (Game|Damage|ApplyDamage _asbp_person (Variables|Default|GetDirectDamage) 0 0)
    (if (> (Math|Random|RandomInteger 100) 50)
      (Transformation|Teleport _returnvalue "2310.000000,2310.000000,190.000000" "0, 0, 0")
      (else
        (Transformation|Teleport _returnvalue "-2130.000000,2610.000000,190.000000" "0, 0, 0")))
    (Utilities|FlowControl|Delay 0.3)
    (Variables|Default|SetIsAttacking false)))

(event EventBeginPlay
  (|CallParentFunction) ; This node is disabled and will not be called.\nDrag off pins to build functionality.
)

(event EventTick
  (params (DeltaSeconds :type Float%20%28single-precision%29))
  ;[1 1 1] Check for Trail Point in Vicinity
  (bind _asbp_person (Utilities|Casting|CastToBP_Person (Game|Player|GetPlayerPawn 0))))

(fn ConstructionScript
  (|CallParentFunction))