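; Player pawn with Enhanced Input movement and look, where damage builds Stress and reaching the maximum sends the player back to the start menu.
; A line trace from the first-person camera opens tagged doors or starts dialogue on actors with C_Dialogue.
; Limited-use items lower Stress, and the player UI widget created on BeginPlay displays incoming speech.
; Debug keys apply self-damage and toggle first- and third-person cameras.
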(event Input|EnhancedActionEvents|EnhancedInputActionIA_Look
  (params (ActionValue :type Vector%202D%20Structure) (ElapsedSeconds :type Float%20%28double-precision%29) (TriggeredSeconds :type Float%20%28double-precision%29) (InputAction :type Input%20Action%20Object%20Reference :default "/Game/BPs/Input/Actions/IA_Look.IA_Look"))
  ;[1 1 1] Camera and Pawn Movement
  (:Triggered
    (Pawn|Input|AddControllerYawInput (* (.x ActionValue) -1.0))
    (Pawn|Input|AddControllerPitchInput (.y ActionValue))))

(event Input|EnhancedActionEvents|EnhancedInputActionIA_Move
  (params (ActionValue :type Vector%202D%20Structure) (ElapsedSeconds :type Float%20%28double-precision%29) (TriggeredSeconds :type Float%20%28double-precision%29) (InputAction :type Input%20Action%20Object%20Reference :default "/Game/BPs/Input/Actions/IA_Move.IA_Move"))
  ;[1 1 1] Camera and Pawn Movement
  (:Triggered
    (Pawn|Input|AddMovementInput (Transformation|GetActorRightVector) (.x ActionValue) false)
    (Pawn|Input|AddMovementInput (Transformation|GetActorForwardVector) (.y ActionValue) false)))

(event Game|Damage|EventAnyDamage
  (params (Damage :type Float%20%28single-precision%29) (DamageType :type Damage%20Type%20Object%20Reference) (InstigatedBy :type Controller%20Object%20Reference) (DamageCauser :type Actor%20Object%20Reference))
  ;[1 1 1] Taking Damage and Death
  (bind _output_get (Variables|Default|SetStress (+ Damage (Variables|Default|GetStress))))
  (if (>= _output_get (Variables|Default|GetMaxStress))
    (CallFunction|PlayerBreakdown)))

(event EventSpeaking
  (params (Dialogue :type String) (TextDelay :type Float%20%28double-precision%29) (IsEnd :type Boolean))
  ;[1 1 1] Interaction Event (ray tracing) F KEY
  ;;[1 1 1] Talk to NPC
  (Default|INCSpeech (Variables|Default|GetPlayerUI) Dialogue TextDelay IsEnd))

(event EventBeginPlay
  ;[1 1 1] Init
  (Utilities|FlowControl|Sequence
    (:then_0
      (Variables|Default|SetIsMaxStress false)
      (Variables|Default|SetStress 0.0)
      (Variables|Default|SetHealthItemUses 10))
    (:then_1
      (CallFunction|UpdatePlayerUI))
    (:then_2
      ;[1 1 1] Camera and Pawn Movement
      (bind _asplayer_controller (Utilities|Casting|CastToPlayerController (Pawn|GetController)))
      (Utilities|IsValid (PlayerController|LocalPlayerSubsystems|GetEnhancedInputLocalPlayerSubsystem _asplayer_controller)
        (:Is%20Valid
          (Input|AddMappingContext (PlayerController|LocalPlayerSubsystems|GetEnhancedInputLocalPlayerSubsystem _asplayer_controller) "/Game/BPs/Input/IMC_Default.IMC_Default" 0 "(bIgnoreAllPressedKeysUntilRelease=True,bForceImmediately=False)"))))))

(event Input|KeyboardEvents|DebugKeyM
  (params (Key :type Key%20Structure :default "None") (ActionValue :type Input%20Action%20Value%20Structure))
  ;[1 1 1] Damage Debug M KEY
  (:Pressed
    (Game|Damage|ApplyDamage self 1e+01 0 0)
    (Components|Animation|PlayAnimation (Variables|Default|Getmeredith_arms) "/Game/Models/meredith/meredith_arms/hand_shake.hand_shake" false)
    (Development|PrintString (Utilities|String|ToString(Float) (Variables|Default|GetStress)))))

(event Input|KeyboardEvents|K
  (params (Key :type Key%20Structure :default "None"))
  ;[1 1 1] Debug Changing POV K KEY
  (:Pressed
    (Utilities|FlowControl|FlipFlop
      (:A
        (Components|Activation|SetActive (Variables|Default|GetFirstP) false false)
        (Components|Activation|SetActive (Variables|Default|GetThirdP) true false)
        (Development|SetHiddeninGame (Variables|Character|GetMesh) false false))
      (:B
        (Components|Activation|SetActive (Variables|Default|GetFirstP) true false)
        (Components|Activation|SetActive (Variables|Default|GetThirdP) false false)
        (Development|SetHiddeninGame (Variables|Character|GetMesh) true false)))))

(event Input|KeyboardEvents|F
  (params (Key :type Key%20Structure :default "None"))
  (bind _firstp (Variables|Default|GetFirstP))
  (bind _returnvalue (Transformation|GetWorldLocation _firstp))
  ;[1 1 1] Interaction Event (ray tracing) F KEY
  (:Pressed
    (bind (_outhit _returnvalue_2) (Collision|LineTraceByChannel _returnvalue (+ _returnvalue (* (Math|Vector|GetForwardVector _firstp) 2.5e+02)) "TraceTypeQuery2" false 0 "None" true "(R=1.000000,G=0.000000,B=0.000000,A=1.000000)" "(R=0.000000,G=1.000000,B=0.000000,A=1.000000)" 1.0))
    (if _returnvalue_2
      ;;[1 1 1] Open/CloseDoor
      (if (Actor|ActorHasTag (.HitActor (Collision|BreakHitResult _outhit)) "Door")
        (bind _asbp_door (Utilities|Casting|CastToBP_Door (.HitActor (Collision|BreakHitResult _outhit))))
        (Default|OpenDoor _asbp_door)
        (else
          ;;[1 1 1] Talk to NPC
          (Utilities|IsValid (Actor|GetComponentbyClass (.HitActor (Collision|BreakHitResult _outhit)) "/Game/BPs/NPCs/C_Dialogue.C_Dialogue_C")
            (:Is%20Valid
              (Default|ActiveSpeaking (Actor|GetComponentbyClass (.HitActor (Collision|BreakHitResult _outhit)) "/Game/BPs/NPCs/C_Dialogue.C_Dialogue_C")))))))))

(event Input|KeyboardEvents|E
  (params (Key :type Key%20Structure :default "None"))
  ;[1 1 1] Using health Item (Limited Uses) E KEY
  (:Pressed
    (if (> (Variables|Default|GetHealthItemUses) 0)
      (Variables|Default|SetHealthItemUses (- (Variables|Default|GetHealthItemUses) 1))
      (if (> (Variables|Default|GetStress) 0.0)
        (Variables|Default|SetStress (- (Variables|Default|GetStress) 1e+01))))))

(fn ConstructionScript)

(fn UpdatePlayerUI
  (bind _returnvalue (UserInterface|CreateWidget "/Game/UI/Widget_PlayerUI.Widget_PlayerUI_C" (Game|GetPlayerController 0)))
  (bind _output_get (Variables|Default|SetPlayerUI _returnvalue))
  (UserInterface|Viewport|AddtoViewport _output_get 0))

(fn PlayerBreakdown
  (Variables|Default|SetIsMaxStress true)
  (Input|DisableInput 0)
  (Game|OpenLevel(byName) "StartMenuMap"))

(fn CheckSpeaking
  (return (Variables|/Game/UI/Widget_PlayerUI.Widget_PlayerUI_C|GetIsLooping (Variables|Default|GetPlayerUI))))